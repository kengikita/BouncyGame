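; Enemy spawner actor that spawns waves of BP_Enemy on a looping five-second timer from BeginPlay.
; Each tick of the timer loops over the EnemySpawned count, printing the index and spawning at the spawner's own transform, adjusting for collision but always spawning.
; A random pick among five world locations is present but disconnected, so it has no effect on spawn position.
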(event `self.ReceiveBeginPlay`
  (`KismetSystemLibrary.K2_SetTimerDelegate` (delegate `Spawn Enemy`) 5.0 true))

(event `Spawn Enemy`
  (for _index (range (`self.EnemySpawned`))
    (`KismetSystemLibrary.PrintString` (`KismetStringLibrary.Conv_IntToString` _index))
    (`|SpawnActorFromClass` "/Game/BP_Enemy.BP_Enemy_C" (`self.GetTransform`) "AdjustIfPossibleButAlwaysSpawn" "OverrideRootScale" null null)))

(fn `UserConstructionScript`)