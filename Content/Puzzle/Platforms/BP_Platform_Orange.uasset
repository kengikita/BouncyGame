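; BP_Platform_Orange is a puzzle platform that detects objects tagged "Orange" resting in its Box trigger.
; On overlap begin it sets OrangeON on the Level_GS game state and calls AllOn, presumably to check whether every platform is active.
; On overlap end it clears OrangeON without calling AllOn, printing a debug string in both cases.
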(event `self.Box.OnComponentBeginOverlap`
  (params (OverlappedComponent :type "PrimitiveComponent Object Reference") (OtherActor :type "Actor Object Reference") (OtherComp :type "PrimitiveComponent Object Reference") (OtherBodyIndex :type Integer) (bFromSweep :type Boolean) (SweepResult :type "HitResult Structure (by ref)"))
  (bind _aslevel_gs (cast `/Game/Level_GS` (`GameplayStatics.GetGameState`)))
  (if (`self.ActorHasTag` OtherActor "Orange")
    (set `/Game/Level_GS.OrangeON` true _aslevel_gs)
    (`KismetSystemLibrary.PrintString` "OrangeON")
    (`/Game/Level_GS.AllOn` _aslevel_gs)))

(event `self.Box.OnComponentEndOverlap`
  (params (OverlappedComponent :type "PrimitiveComponent Object Reference") (OtherActor :type "Actor Object Reference") (OtherComp :type "PrimitiveComponent Object Reference") (OtherBodyIndex :type Integer))
  (bind _aslevel_gs (cast `/Game/Level_GS` (`GameplayStatics.GetGameState`)))
  (if (`self.ActorHasTag` OtherActor "Orange")
    (set `/Game/Level_GS.OrangeON` false _aslevel_gs)
    (`KismetSystemLibrary.PrintString` "OrangeOFF")))

(fn `UserConstructionScript`)