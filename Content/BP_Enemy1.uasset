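; Enemy that constantly turns toward the first-person player and damages them when its PawnSensing spots them.
; A self-calling, short-delay loop interpolates its yaw toward the player, while a long sensing interval paces detection to roughly five seconds.
; Each sighting plays a weapon fire sound and applies damage through the Level_GS game state.
; A retriggerable delay slightly longer than that interval clears the detected flag and plays a missed sound once sightings stop.
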(event `self.ReceiveBeginPlay`
  ;[1 1 1] Look at player and change sensing interval for how long it takes NPC to detect the player
  (bind _asfirst_person_character (cast `/Game/FirstPersonBP/Blueprints/FirstPersonCharacter` (`GameplayStatics.GetPlayerCharacter` 0)))
  (set `self.PlayerReferemce` _asfirst_person_character)
  (`self.FacePlayer`)
  (`PawnSensingComponent.SetSensingInterval` (`self.PawnSensing`) 5.0))

(event `self.PawnSensing.OnSeePawn`
  (params (Pawn :type "Pawn Object Reference"))
  ;[1 1 1] Detects player and deals damage if player in view for 5 seconds
  (set `self.PlayerDetected` true)
  (`|ExecutionSequence`
    (:`then_0`
      (`self.DealDamage`)
      (`GameplayStatics.PlaySound2D` "/Game/FirstPerson/Audio/FirstPersonTemplateWeaponFire02.FirstPersonTemplateWeaponFire02" 1.0 1.0 0.0 null null))
    (:`then_1`
      (`KismetSystemLibrary.RetriggerableDelay` 5.1)
      (set `self.PlayerDetected` false)
      (`GameplayStatics.PlaySound2D` "/Game/Sounds/missed.missed" 1.0 1.0 0.0 null null))))

(event `DealDamage`
  ;[1 1 1] Apply damage to player
  (bind _aslevel_gs (cast `/Game/Level_GS` (`GameplayStatics.GetGameState`)))
  (`/Game/Level_GS.Damage Player` _aslevel_gs 50.0))

(event `FacePlayer`
  (bind (_returnvalue_roll _returnvalue_pitch _returnvalue_yaw) (`KismetMathLibrary.BreakRotator` (`KismetMathLibrary.RInterpTo` (`self.K2_GetActorRotation`) (`KismetMathLibrary.FindLookAtRotation` (`self.K2_GetActorLocation`) (`self.K2_GetActorLocation` (`self.PlayerReferemce`))) (`GameplayStatics.GetWorldDeltaSeconds`) 20.0)))
  ;[1 1 1] Look at player
  (`self.K2_SetActorRotation` (`KismetMathLibrary.MakeRotator` 0.0 0.0 _returnvalue_yaw))
  (`KismetSystemLibrary.Delay` 0.001)
  (`self.FacePlayer`))

(fn `UserConstructionScript`)